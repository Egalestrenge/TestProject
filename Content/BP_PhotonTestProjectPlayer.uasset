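; BP_PhotonTestProjectPlayer is a test player Blueprint that reports Photon networking status through an on-screen debug widget.
; On BeginPlay it creates the widget, then either continues at once if the game instance reports Photon connected, or binds a callback to the connected event.
; Both paths converge on fetching the local Photon player from the game instance's PhotonNetwork, then push connection state, load state and player ID to the widget.
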(event Custom|CustomEvent_0
  (Variables|/Game/WBP_PhotonTestProjectDebug.WBP_PhotonTestProjectDebug_C|SetIsPhotonConnected (Variables|Default|GetDebug) true)
  (Development|PrintString "Loading local player")
  (bind _returnvalue (Class|PhotonNetwork|GetLocalPhotonPlayer (Variables|/Game/PhotonTestProjectGameInstance.PhotonTestProjectGameInstance_C|GetPhotonNetwork (.AsPhoton%20Test%20Project%20Game%20Instance (Utilities|Casting|CastToPhotonTestProjectGameInstance (Game|GetGameInstance))))))
  (Development|PrintString "Local Player Loaded")
  (Variables|/Game/WBP_PhotonTestProjectDebug.WBP_PhotonTestProjectDebug_C|SetIsLocalPlayerLoadedFromPhoton (Variables|Default|GetDebug) true)
  (bind _returnvalue_2 (Class|PhotonPlayer|GetId _returnvalue))
  (Variables|/Game/WBP_PhotonTestProjectDebug.WBP_PhotonTestProjectDebug_C|SetLocalPlayerID (Variables|Default|GetDebug) _returnvalue_2))

(event EventBeginPlay
  (bind _returnvalue (Game|GetGameInstance))
  (bind _asphoton_test_project_game_instance (Utilities|Casting|CastToPhotonTestProjectGameInstance _returnvalue))
  (bind _returnvalue_2 (UserInterface|CreateWidget "/Game/WBP_PhotonTestProjectDebug.WBP_PhotonTestProjectDebug_C"))
  (bind _output_get (Variables|Default|SetDebug _returnvalue_2))
  (UserInterface|Viewport|AddtoViewport _output_get 0)
  (if (Variables|/Game/PhotonTestProjectGameInstance.PhotonTestProjectGameInstance_C|GetIsPhotonConnected _asphoton_test_project_game_instance)
    (Variables|/Game/WBP_PhotonTestProjectDebug.WBP_PhotonTestProjectDebug_C|SetIsPhotonConnected (Variables|Default|GetDebug) true)
    (Development|PrintString "Loading local player")
    (bind _returnvalue_3 (Class|PhotonNetwork|GetLocalPhotonPlayer (Variables|/Game/PhotonTestProjectGameInstance.PhotonTestProjectGameInstance_C|GetPhotonNetwork _asphoton_test_project_game_instance)))
    (Development|PrintString "Local Player Loaded")
    (Variables|/Game/WBP_PhotonTestProjectDebug.WBP_PhotonTestProjectDebug_C|SetIsLocalPlayerLoadedFromPhoton (Variables|Default|GetDebug) true)
    (bind _returnvalue_4 (Class|PhotonPlayer|GetId _returnvalue_3))
    (Variables|/Game/WBP_PhotonTestProjectDebug.WBP_PhotonTestProjectDebug_C|SetLocalPlayerID (Variables|Default|GetDebug) _returnvalue_4)
    (else
      (EventDispatchers|BindEventtoPhotonConnected _asphoton_test_project_game_instance (delegate Custom|CustomEvent_0)))))

(event Collision|EventActorBeginOverlap
  (params (OtherActor :type Actor%20Object%20Reference)))

(event EventTick
  (params (DeltaSeconds :type Float%20%28single-precision%29)))

(fn ConstructionScript)